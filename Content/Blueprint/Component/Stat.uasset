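; Stat component that manages a character's life and mana, including regeneration, damage and death.
; Setup fills both pools from maximums derived from Strength, Stamina and Intelligence, which are recomputed every Tick.
; Tick also drives timed regeneration from bonus stats, skipping any increment that would exceed the maximum.
; GiveDamage damages a target Stat and applies life steal by passing negative damage to its own TakeDamage.
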(event EventTick
  (params (DeltaSeconds :type Float%20%28single-precision%29))
  (CallFunction|Generation DeltaSeconds)
  (CallFunction|SetMax))

(event EventInitializeComponent
  (CallFunction|Setup))

(fn LifeGeneration
  (params (Time :type Float%20%28single-precision%29 :default 0.0))
  (bind _stats (Variables|Default|GetStats))
  (bind _returnvalue (* (.life_amplifier (.bonus _stats)) (.life_regeneration (.bonus _stats))))
  (bind _returnvalue_2 (* (.life_regeneration_speed (.bonus _stats)) (.life_regeneration_speed_amplifier (.bonus _stats))))
  (bind _returnvalue_3 (Math|Float|Floor _returnvalue))
  (Variables|Default|SetLife%20Timer (+ Time (Variables|Default|GetLife%20Timer)))
  (if (>= (Variables|Default|GetLife%20Timer) _returnvalue_2)
    (Variables|Display|SetLife%20per%20Sec (Utilities|String|ToString(Float) (/ (Math|Conversions|ToFloat(Integer) (+ (.life_regeneration_bonus (.bonus _stats)) _returnvalue_3)) _returnvalue_2)))
    (Variables|Default|SetLife%20Timer 0.0)
    (if (and (<= (+ (Variables|Base|GetCurrent%20Life) _returnvalue_3 (.life_regeneration_bonus (.bonus _stats))) (Variables|Base|GetMax%20Life)) (Variables|Default|GetLife%20Generation%20Toggle))
      (Variables|Base|SetCurrent%20Life (+ (Variables|Base|GetCurrent%20Life) _returnvalue_3 (.life_regeneration_bonus (.bonus _stats)))))))

(fn ManaGeneration
  (params (Timer :type Float%20%28single-precision%29 :default 0.0))
  (bind _stats (Variables|Default|GetStats))
  (bind _returnvalue (* (.mana_amplifier (.bonus _stats)) (.mana_regeneration (.bonus _stats))))
  (bind _returnvalue_2 (* (.mana_regeneration_speed (.bonus _stats)) (.mana_regeneration_speed_amplifier (.bonus _stats))))
  (bind _returnvalue_3 (Math|Float|Floor _returnvalue))
  (Variables|Default|SetMana%20Timer (+ Timer (Variables|Default|GetMana%20Timer)))
  (if (>= (Variables|Default|GetMana%20Timer) _returnvalue_2)
    (Variables|Default|SetMana%20Timer 0.0)
    (Variables|Display|SetMana%20per%20Sec (Utilities|String|ToString(Float) (/ (Math|Conversions|ToFloat(Integer) (+ (.mana_regeneration_bonus (.bonus _stats)) _returnvalue_3)) _returnvalue_2)))
    (if (and (<= (+ (Variables|Base|GetCurrent%20Mana) _returnvalue_3 (.mana_regeneration_bonus (.bonus _stats))) (Variables|Base|GetMax%20Mana)) (Variables|Default|GetMana%20Generation%20Toggle))
      (Variables|Base|SetCurrent%20Mana (+ (Variables|Base|GetCurrent%20Mana) _returnvalue_3 (.mana_regeneration_bonus (.bonus _stats)))))))

(fn TakeDamage
  (params (Damage :type Integer))
  (if (>= (Variables|Base|GetCurrent%20Life) Damage)
    (if (>= (Variables|Base|GetCurrent%20Life) (Variables|Base|GetMax%20Life))
      (Variables|Base|SetCurrent%20Life (Variables|Base|GetMax%20Life))
      (else
        (LocalVariables|SetTaken%20Damage Damage)
        (Variables|Base|SetCurrent%20Life (- (Variables|Base|GetCurrent%20Life) Damage))
        (return (LocalVariables|GetTaken%20Damage))))
    (else
      (LocalVariables|SetTaken%20Damage (- Damage (Variables|Base|GetCurrent%20Life)))
      (Variables|Base|SetCurrent%20Life 0)
      (Variables|Base|SetDead true)
      (Development|PrintString "Loser")
      (return (LocalVariables|GetTaken%20Damage)))))

(fn GiveDamage
  (params (Target :type Actor%20Object%20Reference) (Damage :type Integer))
  (bind _asstat (Utilities|Casting|CastToStat Target))
  (bind _damage_taken (CallFunction|TakeDamage _asstat Damage))
  (CallFunction|TakeDamage (Math|Float|Floor (* (- 0 _damage_taken) (.life_steal (.secondary (Variables|Default|GetStats)))))))

(fn Generation
  (params (time :type Float%20%28single-precision%29 :default 0.0))
  (bind _stats (Variables|Default|GetStats))
  (Variables|Display|SetLife%20per%20Sec (Utilities|String|ToString(Float) (/ (Math|Conversions|ToFloat(Integer) (+ (.life_regeneration_bonus (.bonus _stats)) (Math|Float|Floor (* (.life_amplifier (.bonus _stats)) (.life_regeneration (.bonus _stats)))))) (* (.life_regeneration_speed (.bonus _stats)) (.life_regeneration_speed_amplifier (.bonus _stats))))))
  (Variables|Display|SetMana%20per%20Sec (Utilities|String|ToString(Float) (/ (Math|Conversions|ToFloat(Integer) (+ (.mana_regeneration_bonus (.bonus _stats)) (Math|Float|Floor (* (.mana_amplifier (.bonus _stats)) (.mana_regeneration (.bonus _stats)))))) (* (.mana_regeneration_speed (.bonus _stats)) (.mana_regeneration_speed_amplifier (.bonus _stats))))))
  (CallFunction|LifeGeneration time)
  (CallFunction|ManaGeneration time))

(fn SetMax
  (bind _stats (Variables|Default|GetStats))
  (bind _returnvalue (* (.stamina (.primary _stats)) 2))
  (Variables|Base|SetMax%20Life (* (* (.stength (.primary _stats)) 5) _returnvalue))
  (Variables|Base|SetMax%20Mana (* _returnvalue (* (.intelligence (.primary _stats)) 5))))

(fn Setup
  (CallFunction|SetMax)
  (Variables|Base|SetCurrent%20Life (Variables|Base|GetMax%20Life))
  (Variables|Base|SetCurrent%20Mana (Variables|Base|GetMax%20Mana)))