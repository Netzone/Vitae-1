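; Spell-casting component that spawns the selected spell's actor at its owner, passing power, owner and lifespan.
; Button release checks cooldown and mana, or life for Blood Magic, then starts a Haste-scaled cast timer.
; Tick counts down cooldowns and casts, cancelling when owner velocity exceeds Focus tolerance; completion deducts cost and starts cooldown.
; Channeling is an empty stub, and targeting-decal code is unconnected.
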(event Custom|Set%20Cast%20Timer
  (bind _stats (Variables|Default|GetStats))
  (bind _spell_list (Variables|Default|GetSpell%20List))
  (bind _selected_spell (Variables|Default|GetSelected%20Spell))
  (bind _item (Utilities|Array|Get(acopy) _spell_list _selected_spell))
  (bind _returnvalue (* (.casttime _item) (.haste (.secondary _stats))))
  ;[1 1 1] Cast Setup
  (if (.blood_magic _item)
    (if (> (Variables|Default|GetCurrent%20Life) (.mana _item))
      (if (and (<= (Utilities|Array|Get(acopy) (Variables|Default|GetCurrent%20Cooldown) _selected_spell) 0.0) (not (Variables|Cast|GetCast))) :!label _label
        (Variables|Default|SetMana%20Generation%20Toggle false)
        (Variables|Cast|SetCast%20Time _returnvalue)
        (Variables|Cast|SetMax%20Cast%20Time _returnvalue)
        (Variables|Cast|SetCast true)
        (Development|PrintString (Utilities|String|Append (Utilities|String|Append (Utilities|String|Append (Utilities|String|Append "Casting: " (Utilities|String|ToString(Name) (.name _item))) " in ") (Utilities|String|ToString(Float) _returnvalue)) "sec"))
        (else
          (Development|PrintString "Unable to Cast")))
      (else
        (Development|PrintString "Need more health!")))
    (elif (>= (Variables|Default|GetCurrent%20Mana) (.mana _item))
      (goto _label)
      (else
        (Development|PrintString "Need more mana")))))

(event Custom|Spell%20Trigger
  (bind _returnvalue (Components|GetOwner))
  (bind _spell_list (Variables|Default|GetSpell%20List))
  (bind _selected_spell (Variables|Default|GetSelected%20Spell))
  (bind _item (Utilities|Array|Get(acopy) _spell_list _selected_spell))
  ;[1 1 1] Spell Triggerd
  (if (.blood_magic _item)
    (Variables|Default|SetCurrent%20Life (- (Variables|Default|GetCurrent%20Life) (.mana _item)))
    (else
      (Variables|Default|SetCurrent%20Mana (- (Variables|Default|GetCurrent%20Mana) (.mana _item)))))
  (bind _returnvalue_2 (Game|SpawnActorfromClass (.magic_bp _item) (Math|Conversions|ToTransform(Vector) (Transformation|GetActorLocation (Components|GetOwner))) false 0))
  (Development|PrintString (Utilities|GetDisplayName _returnvalue))
  (Variables|/Game/Blueprint/Component/Spell.Spell_C|SetPower (Utilities|Array|Get(acopy) (Actor|GetComponentsByClass _returnvalue_2 "/Game/Blueprint/Component/Spell.Spell_C")) (.power _item))
  (Variables|/Game/Blueprint/Component/Spell.Spell_C|SetActor%20Owner (Utilities|Array|Get(acopy) (Actor|GetComponentsByClass _returnvalue_2 "/Game/Blueprint/Component/Spell.Spell_C")) _returnvalue)
  (Variables|/Game/Blueprint/Component/Spell.Spell_C|SetLife%20Span (Utilities|Array|Get(acopy) (Actor|GetComponentsByClass _returnvalue_2 "/Game/Blueprint/Component/Spell.Spell_C")) (.lifespan _item))
  (Utilities|Array|SetArrayElem (Variables|Default|GetCurrent%20Cooldown) (Variables|Default|GetSelected%20Spell) (.cooldown _item) true) ; Set Cooldown
)

(event Custom|Set%20Target%20Type
  ;[1 1 1] Decals
  (switch Utilities|FlowControl|Switch|Switchonenum_magic_target "NewEnumerator2"))

(event Custom|Channel
  ;[1 1 1] Channel
  (if (.channel (Utilities|Array|Get(acopy) (Variables|Default|GetSpell%20List) (Variables|Default|GetSelected%20Spell)))
    _))

(event Custom|Action%20Release
  (params (Action :type Integer :default 0))
  ;[1 1 1] Check Button Up and run selected attack
  (Variables|Default|SetSelected%20Spell Action)
  (CallFunction|SetCastTimer)
  (Variables|Default|SetDown false))

(event Custom|Action%20Press
  (params (Action :type Integer :default 0))
  ;[1 1 1] Check Button Down and charge selected attack
  (Variables|Default|SetSelected%20Spell Action)
  (CallFunction|Channel)
  (Variables|Default|SetShow%20Decal true)
  (Variables|Default|SetDown true))

(event EventTick
  (params (DeltaSeconds :type Float%20%28single-precision%29))
  (bind _returnvalue (Components|GetOwner))
  (bind _returnvalue_2 (Transformation|GetVelocity _returnvalue))
  (CallFunction|SetMax)
  (if (Variables|Default|GetShow%20Decal)
    (CallFunction|SetTargetType))
  (CallFunction|Generation DeltaSeconds)
  ;[1 1 1] Cooldown Timer
  (for (_array_element _array_index) (Variables|Default|GetCurrent%20Cooldown)
    (if (>= _array_element 0.0)
      (Utilities|Array|SetArrayElem (Variables|Default|GetCurrent%20Cooldown) _array_index (- _array_element DeltaSeconds) true)))
  ;[1 1 1] Cast Timer
  (if (Math|Boolean|ANDBoolean (Variables|Cast|GetCast) (Math|Float|NearlyEqual(Float) (+ (.x _returnvalue_2) (.y _returnvalue_2) (.z _returnvalue_2)) 0.0 (.focus (.secondary (Variables|Default|GetStats)))) (>= (Variables|Cast|GetMax%20Cast%20Time) 0.0))
    (bind _output_get (Variables|Cast|SetCast%20Time (- (Variables|Cast|GetCast%20Time) DeltaSeconds)))
    (if (<= _output_get 0.0) ; If cast time is zero, trigger spell
      (Variables|Cast|SetMax%20Cast%20Time -0.1)
      (CallFunction|SpellTrigger))
    (else
      (Variables|Cast|SetMax%20Cast%20Time -0.1)
      (Variables|Cast|SetCast false)
      (Variables|Default|SetMana%20Generation%20Toggle true)
      (if (not (Variables|Default|GetDown))
        (Variables|Default|SetShow%20Decal false)))))

(event EventInitializeComponent
  ;[1 1 1] Init
  (Utilities|Array|Resize (Variables|Default|GetCurrent%20Cooldown) (Utilities|Array|Length (Variables|Default|GetSpell%20List)))
  (CallFunction|Setup))